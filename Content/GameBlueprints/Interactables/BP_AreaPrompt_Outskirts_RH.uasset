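; One-shot area prompt trigger that shows the Outskirts title image on the HUD when the melee player character enters its sphere.
; On first overlap, it reaches the HUD through the player controller, plays the Outskirts fade-in animation and makes the image visible.
; When the character fully leaves, it plays the same animation in reverse and destroys itself, so the prompt does not repeat.
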(event `self.Sphere.OnComponentBeginOverlap`
  (params (OverlappedComponent :type "PrimitiveComponent Object Reference") (OtherActor :type "Actor Object Reference") (OtherComp :type "PrimitiveComponent Object Reference") (OtherBodyIndex :type Integer) (bFromSweep :type Boolean) (SweepResult :type "HitResult Structure (by ref)"))
  (bind _asbp_melee_player_character_rh (cast `/Game/GameBlueprints/Characters/PlayerCharacters/BP_MeleePlayerCharacter_RH` OtherActor))
  (if (`self.IsOverlappingActor` _asbp_melee_player_character_rh)
    (bind _asbp_player_controller_rh (cast `/Game/GameBlueprints/GameManagers/BP_PlayerController_RH` (`GameplayStatics.GetPlayerController` 0)))
    (`/Engine/EditorBlueprintResources/StandardMacros.DoOnce` false
      (:`Completed`
        (bind _hudref (`/Game/GameBlueprints/GameManagers/BP_PlayerController_RH.HUDRef` _asbp_player_controller_rh))
        (`UserWidget.PlayAnimation` _hudref (`/Game/UI/WBP_HUD_RH.FadeInOutskirts` _hudref) 0.0 1 "Forward" 1.0 false)
        (`Widget.SetVisibility` (`/Game/UI/WBP_HUD_RH.OutskirtsImage` _hudref) "Visible")))))

(event `self.Sphere.OnComponentEndOverlap`
  (params (OverlappedComponent :type "PrimitiveComponent Object Reference") (OtherActor :type "Actor Object Reference") (OtherComp :type "PrimitiveComponent Object Reference") (OtherBodyIndex :type Integer))
  (bind _asbp_melee_player_character_rh (cast `/Game/GameBlueprints/Characters/PlayerCharacters/BP_MeleePlayerCharacter_RH` OtherActor))
  (if (not (`self.IsOverlappingActor` _asbp_melee_player_character_rh))
    (bind _asbp_player_controller_rh (cast `/Game/GameBlueprints/GameManagers/BP_PlayerController_RH` (`GameplayStatics.GetPlayerController` 0)))
    (bind _hudref (`/Game/GameBlueprints/GameManagers/BP_PlayerController_RH.HUDRef` _asbp_player_controller_rh))
    (`UserWidget.PlayAnimation` _hudref (`/Game/UI/WBP_HUD_RH.FadeInOutskirts` _hudref) 0.0 1 "Reverse" 1.0 false)
    (`Widget.SetVisibility` (`/Game/UI/WBP_HUD_RH.OutskirtsImage` _hudref) "Visible")
    (`self.K2_DestroyActor`)))

(fn `UserConstructionScript`)