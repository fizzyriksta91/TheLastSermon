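; BP_LevelChanger_RH is an interactable that plays dialogue and can send players to the Outskirts level.
; Its interaction sphere shows or hides a keyboard billboard for the melee character and a controller billboard for the ranged character.
; Interact begins dialogue on the dialogue component, then immediately checks its EndDialogue flag and opens Outskirts only if that is already true.
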(event `self.InteractionSphere.OnComponentBeginOverlap`
  (params (OverlappedComponent :type "PrimitiveComponent Object Reference") (OtherActor :type "Actor Object Reference") (OtherComp :type "PrimitiveComponent Object Reference") (OtherBodyIndex :type Integer) (bFromSweep :type Boolean) (SweepResult :type "HitResult Structure (by ref)"))
  ; Display Interact prompt
  (`|ExecutionSequence`
    (:`then_0`
      (bind _asbp_melee_player_character_rh (cast `/Game/GameBlueprints/Characters/PlayerCharacters/BP_MeleePlayerCharacter_RH` OtherActor))
      (if (`self.IsOverlappingActor` _asbp_melee_player_character_rh)
        (`SceneComponent.SetVisibility` (`self.BillboardKeyboard`) true false)))
    (:`then_1`
      (bind _asbp_range_player_character_rh (cast `/Game/GameBlueprints/Characters/PlayerCharacters/BP_RangePlayerCharacter_RH` OtherActor))
      (if (`self.IsOverlappingActor` _asbp_range_player_character_rh)
        (`SceneComponent.SetVisibility` (`self.BillboardController`) true false)))))

(event `self.InteractionSphere.OnComponentEndOverlap`
  (params (OverlappedComponent :type "PrimitiveComponent Object Reference") (OtherActor :type "Actor Object Reference") (OtherComp :type "PrimitiveComponent Object Reference") (OtherBodyIndex :type Integer))
  ; Remove Interact prompt
  (`|ExecutionSequence`
    (:`then_0`
      (bind _asbp_melee_player_character_rh (cast `/Game/GameBlueprints/Characters/PlayerCharacters/BP_MeleePlayerCharacter_RH` OtherActor))
      (if (not (`self.IsOverlappingActor` _asbp_melee_player_character_rh))
        (`SceneComponent.SetVisibility` (`self.BillboardKeyboard`) false false)))
    (:`then_1`
      (bind _asbp_range_player_character_rh (cast `/Game/GameBlueprints/Characters/PlayerCharacters/BP_RangePlayerCharacter_RH` OtherActor))
      (if (not (`self.IsOverlappingActor` _asbp_range_player_character_rh))
        (`SceneComponent.SetVisibility` (`self.BillboardController`) false false)))))

(event `self.Interact`
  (params (InteractingActor :type "BaseCharacter Object Reference"))
  (bind _bpc_dialoguecomponent_rh (`self.BPC_DialogueComponent_RH`))
  (`/Game/GameBlueprints/DialogueSystem/BPC_DialogueComponent_RH.BeginDialogue` _bpc_dialoguecomponent_rh)
  (if (`/Game/GameBlueprints/DialogueSystem/BPC_DialogueComponent_RH.EndDialogue?` _bpc_dialoguecomponent_rh)
    (`GameplayStatics.OpenLevel` "Outskirts")))

(fn `UserConstructionScript`)