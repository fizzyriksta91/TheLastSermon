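; Player camera manager that can set up a single shared camera for the game.
; SetUpSharedCamera runs only for player controller ID 0, spawning a rotated BP_SharedCamera_RH, storing it in CamerRef and making it player 0's view target.
; BeginPlay is empty and the only setup call in this graph is disconnected.
; BlueprintUpdateCamera returns false, leaving camera updates to the default logic.
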(event `self.ReceiveBeginPlay`)

(event `SetUpSharedCamera`
  (if (== (`GameplayStatics.GetPlayerControllerID` (`self.GetOwningPlayerController`)) 0)
    (bind _returnvalue (`|SpawnActorFromClass` "/Game/GameBlueprints/CameraSystem/BP_SharedCamera_RH.BP_SharedCamera_RH_C" (`KismetMathLibrary.MakeTransform` (0.0 0.0 0.0) (struct :`Pitch` 40.0 :`Yaw` 45.0)) "Undefined" "MultiplyWithRoot" null null))
    (set `self.CamerRef` _returnvalue)
    (`PlayerController.SetViewTargetWithBlend` (`GameplayStatics.GetPlayerController` 0) (`self.CamerRef`) 0.0 "VTBlend_Linear" 0.0 false)))

(fn `BlueprintUpdateCamera`
  (params (CameraTarget :type "Actor Object Reference"))
  (returns (NewCameraLocation :type "Vector Structure") (NewCameraRotation :type "Rotator Structure") (NewCameraFOV :type "Float (single-precision)") (ReturnValue :type Boolean))
  (return (0.0 0.0 0.0) (struct) 0.0 false))

(fn `UserConstructionScript`)