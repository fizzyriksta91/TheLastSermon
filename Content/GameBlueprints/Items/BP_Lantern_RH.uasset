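; BP_Lantern_RH is a lantern item that tells the two player characters' LanternDamageComp when its light is entered or exited.
; Its Sphere's begin and end overlap events call EnterLight or ExitLight, passing the lantern itself.
; Each event fetches player 0 as melee and player 1 as ranged without checking the overlapping actor, so any overlap notifies both.
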(event `self.Sphere.OnComponentBeginOverlap`
  (params (OverlappedComponent :type "PrimitiveComponent Object Reference") (OtherActor :type "Actor Object Reference") (OtherComp :type "PrimitiveComponent Object Reference") (OtherBodyIndex :type Integer) (bFromSweep :type Boolean) (SweepResult :type "HitResult Structure (by ref)"))
  (`|ExecutionSequence`
    (:`then_0`
      (bind _asbp_melee_player_character_rh (cast `/Game/GameBlueprints/Characters/PlayerCharacters/BP_MeleePlayerCharacter_RH` (`GameplayStatics.GetPlayerCharacter` 0)))
      (bind _output_get (set `self.MeleePlayerRef` _asbp_melee_player_character_rh))
      (`/Engine/EditorBlueprintResources/StandardMacros.IsValid` _output_get
        (:`Is Valid`
          (`LanternDamageComponentRH.EnterLight` (`MeleePlayerCharacterRH.LanternDamageComp` (`self.MeleePlayerRef`)) self))))
    (:`then_1`
      (bind _asbp_range_player_character_rh (cast `/Game/GameBlueprints/Characters/PlayerCharacters/BP_RangePlayerCharacter_RH` (`GameplayStatics.GetPlayerCharacter` 1)))
      (bind _output_get_2 (set `self.RangePlayerRef` _asbp_range_player_character_rh))
      (`/Engine/EditorBlueprintResources/StandardMacros.IsValid` _output_get_2
        (:`Is Valid`
          (`LanternDamageComponentRH.EnterLight` (`RangePlayerCharacterRH.LanternDamageComp` (`self.RangePlayerRef`)) self))))))

(event `self.Sphere.OnComponentEndOverlap`
  (params (OverlappedComponent :type "PrimitiveComponent Object Reference") (OtherActor :type "Actor Object Reference") (OtherComp :type "PrimitiveComponent Object Reference") (OtherBodyIndex :type Integer))
  (`|ExecutionSequence`
    (:`then_0`
      (bind _asbp_melee_player_character_rh (cast `/Game/GameBlueprints/Characters/PlayerCharacters/BP_MeleePlayerCharacter_RH` (`GameplayStatics.GetPlayerCharacter` 0)))
      (bind _output_get (set `self.MeleePlayerRef` _asbp_melee_player_character_rh))
      (`/Engine/EditorBlueprintResources/StandardMacros.IsValid` _output_get
        (:`Is Valid`
          (`LanternDamageComponentRH.ExitLight` (`MeleePlayerCharacterRH.LanternDamageComp` (`self.MeleePlayerRef`)) self))))
    (:`then_1`
      (bind _asbp_range_player_character_rh (cast `/Game/GameBlueprints/Characters/PlayerCharacters/BP_RangePlayerCharacter_RH` (`GameplayStatics.GetPlayerCharacter` 1)))
      (bind _output_get_2 (set `self.RangePlayerRef` _asbp_range_player_character_rh))
      (`/Engine/EditorBlueprintResources/StandardMacros.IsValid` _output_get_2
        (:`Is Valid`
          (`LanternDamageComponentRH.ExitLight` (`RangePlayerCharacterRH.LanternDamageComp` (`self.RangePlayerRef`)) self))))))

(fn `UserConstructionScript`)