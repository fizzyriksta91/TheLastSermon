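; Actor component that runs data-table-driven dialogue, showing speaker names and lines in a dialogue widget.
; Each BeginDialogue call creates or updates the widget from the current row, which supplies the next row, table and end flag.
; When the end flag is set or LeaveDialogue fires, it removes the widget and unlocks movement for the melee and range player characters.
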(event `LeaveDialogue`
  (bind _widgetref (`self.WidgetRef`))
  ; End Dialogue and unlock movement
  (`/Engine/EditorBlueprintResources/StandardMacros.IsValid` _widgetref :!label _label
    (:`Is Valid`
      (`Widget.RemoveFromParent` _widgetref)
      (set `self.EndDialogue?` false)
      (set `self.WidgetRef` null)
      (`|ExecutionSequence`
        (:`then_0`
          (bind _asbp_melee_player_character_rh (cast `/Game/GameBlueprints/Characters/PlayerCharacters/BP_MeleePlayerCharacter_RH` (`GameplayStatics.GetPlayerCharacter` 0)))
          (`BaseCharacter.UnlockMovement` _asbp_melee_player_character_rh))
        (:`then_1`
          (bind _asbp_range_player_character_rh (cast `/Game/GameBlueprints/Characters/PlayerCharacters/BP_RangePlayerCharacter_RH` (`GameplayStatics.GetPlayerCharacter` 1)))
          (`BaseCharacter.UnlockMovement` _asbp_range_player_character_rh))))))

(event `BeginDialogue`
  (if (`self.EndDialogue?`)
    (goto _label)
    (else
      (`/Engine/EditorBlueprintResources/StandardMacros.IsValid` (`self.WidgetRef`)
        (:`Is Valid`
          ; Cycle through dialogue options
          (bind _returnvalue (`|GetDataTableRow` (`self.Data Table`) (`self.Row Name`))
            (:`then`
              (bind (_dialogue _charactername _row _datatable _enddialogue_) (break `/Game/GameBlueprints/DialogueSystem/S_Dialogue_RH` _returnvalue))
              (`/Game/GameBlueprints/DialogueSystem/WBP_Dialogue_RH.Update Dialogue` (`self.WidgetRef`) _dialogue _charactername)
              (set `self.Row Name` _row)
              (set `self.Data Table` _datatable)
              (set `self.EndDialogue?` _enddialogue_))))
        (:`Is Not Valid`
          ; Add dialogue widget to viewport
          (bind _returnvalue_2 (`|GetDataTableRow` (`self.Data Table`) (`self.Row Name`))
            (:`then`
              (bind (_dialogue_2 _charactername_2 _row_2 _datatable_2 _enddialogue__2) (break `/Game/GameBlueprints/DialogueSystem/S_Dialogue_RH` _returnvalue_2))
              (bind _returnvalue_3 (`|CreateWidget` "/Game/GameBlueprints/DialogueSystem/WBP_Dialogue_RH.WBP_Dialogue_RH_C" null _charactername_2 _dialogue_2))
              (bind _output_get (set `self.WidgetRef` _returnvalue_3))
              (`UserWidget.AddToViewport` _output_get 0)
              (set `self.Row Name` _row_2)
              (set `self.Data Table` _datatable_2)
              (set `self.EndDialogue?` _enddialogue__2))))))))