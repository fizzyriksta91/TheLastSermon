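; BP_SharedCamera_RH is a shared multiplayer camera actor that follows the players and zooms with their spread.
; Each tick it moves itself to the average location of all player pawns.
; It then maps a distance from that center through a clamped zoom range, scaled by the minimum arm length, to set the spring arm length.
; The distance loop only measures player 0's pawn, so other players' distances do not affect zoom.
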(event `self.ReceiveTick`
  (params (DeltaSeconds :type "Float (single-precision)"))
  (bind _returnvalue (`KismetMathLibrary.Vector_Distance` (`self.K2_GetActorLocation`) (`self.K2_GetActorLocation` (`GameplayStatics.GetPlayerPawn` 0))))
  (bind _returnvalue_2 (`GameModeBase.GetNumPlayers` (`GameplayStatics.GetGameMode`)))
  (set `self.LocationsSum` (0.0 0.0 0.0))
  (for _index (range _returnvalue_2)
    (set `self.LocationsSum` (+ (`self.LocationsSum`) (`self.K2_GetActorLocation` (`GameplayStatics.GetPlayerPawn` _index)))))
  (`self.K2_SetActorLocation` (/ (`self.LocationsSum`) _returnvalue_2))
  (set `self.DistanceFromCenterPoint` 0.0)
  (bind _returnvalue_3 (`GameModeBase.GetNumPlayers` (`GameplayStatics.GetGameMode`)))
  (set `self.LocationsSum` (0.0 0.0 0.0))
  (for _ (range _returnvalue_3)
    (if (> _returnvalue (`self.DistanceFromCenterPoint`))
      (set `self.DistanceFromCenterPoint` _returnvalue)))
  (set `SpringArmComponent.TargetArmLength` (* (`KismetMathLibrary.MapRangeClamped` (`self.DistanceFromCenterPoint`) (`self.MinDistanceFromCenterPoint`) (`self.MaxDistanceFromCenterPoint`) (`self.MinZoom`) (`self.MaxZoom`)) (`self.MinArmLength`)) (`self.SpringArmComponent`)))

(fn `UserConstructionScript`)