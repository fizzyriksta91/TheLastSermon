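; End-game trigger actor that shows the end screen when a BaseCharacter overlaps its sphere.
; The overlap creates a WBP_EndGame_RH widget, adds it to the viewport, switches player 0 to Game and UI input, and shows the mouse cursor.
; After a short delay it gives the restart button keyboard focus and then pauses the game.
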(event `self.Sphere.OnComponentBeginOverlap`
  (params (OverlappedComponent :type "PrimitiveComponent Object Reference") (OtherActor :type "Actor Object Reference") (OtherComp :type "PrimitiveComponent Object Reference") (OtherBodyIndex :type Integer) (bFromSweep :type Boolean) (SweepResult :type "HitResult Structure (by ref)"))
  (bind _returnvalue (`GameplayStatics.GetPlayerController` 0))
  (bind _endwidgetref (`self.EndWidgetRef`))
  (cast `BaseCharacter` OtherActor)
  (bind _returnvalue_2 (`|CreateWidget` "/Game/UI/WBP_EndGame_RH.WBP_EndGame_RH_C"))
  (bind _output_get (set `self.EndWidgetRef` _returnvalue_2))
  (`UserWidget.AddToViewport` _output_get 0)
  (`WidgetBlueprintLibrary.SetInputMode_GameAndUIEx` _returnvalue _endwidgetref "LockInFullscreen")
  (set `PlayerController.bShowMouseCursor` true _returnvalue)
  (`KismetSystemLibrary.Delay` 0.2)
  (`Widget.SetKeyboardFocus` (`/Game/UI/WBP_EndGame_RH.RestartButton` _endwidgetref))
  (`GameplayStatics.SetGamePaused` true))

(fn `UserConstructionScript`)