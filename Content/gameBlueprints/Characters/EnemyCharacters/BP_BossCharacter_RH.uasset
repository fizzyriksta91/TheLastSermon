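; BP_BossCharacter_RH is a boss enemy character that takes damage and performs montage-driven attacks.
; Any damage received is passed to StatsComp to reduce health.
; KickCombo1 and NormalKick events each play a kick montage and call OnAttackEnd when it completes or is interrupted.
; AOETrail plays the AOE attack montage, but its notify switch has no actions and it never signals attack end.
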(event `self.ReceiveAnyDamage`
  (params (Damage :type "Float (single-precision)") (DamageType :type "DamageType Object Reference") (InstigatedBy :type "Controller Object Reference") (DamageCauser :type "Actor Object Reference"))
  (`StatsComponentRH.ReduceHealth` (`self.StatsComp`) Damage))

(event `KickCombo1`
  (`|PlayMontage` (`self.Mesh`) "/Game/RetargetAnimations/Melee/Combo_Kick_Montage.Combo_Kick_Montage"
    (:`OnCompleted`
      _)
    (:`OnInterrupted`
      _))
  (`self.OnAttackEnd`))

(event `NormalKick`
  (`|PlayMontage` (`self.Mesh`) "/Game/RetargetAnimations/Melee/Mma_Kick_Montage.Mma_Kick_Montage"
    (:`OnCompleted`
      _)
    (:`OnInterrupted`
      _))
  (`self.OnAttackEnd`))

(event `AOETrail`
  (bind _notifyname (`|PlayMontage` (`self.Mesh`) "/Game/RetargetAnimations/Magic/Montage_AOEAttack.Montage_AOEAttack")
    (:`OnNotifyBegin`
      (switch `name` _notifyname))))

(fn `UserConstructionScript`)