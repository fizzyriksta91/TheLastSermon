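; Game mode for local two-player play that gives the first player a melee character and the other a ranged one.
; BeginPlay creates the second player once, using a PlayerInitialised flag on BP_GameInstance_RH to prevent repeats.
; The SpawnDefaultPawnFor override picks the class by controller ID, then spawns and possesses it at the start spot.
; That override returns the ranged character variable even on the melee branch.
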(event `self.ReceiveBeginPlay`
  (bind _asbp_game_instance_rh (cast `/Game/GameBlueprints/GameManagers/BP_GameInstance_RH` (`GameplayStatics.GetGameInstance`)))
  (if (== (`/Game/GameBlueprints/GameManagers/BP_GameInstance_RH.PlayerInitialised` _asbp_game_instance_rh) false)
    (`self.SpawnSecondPlayer`)
    (set `/Game/GameBlueprints/GameManagers/BP_GameInstance_RH.PlayerInitialised` true _asbp_game_instance_rh)))

(event `SpawnSecondPlayer`
  (set `self.DefaultPawnClass` "/Script/CS2Project.RangePlayerCharacterRH")
  (`GameplayStatics.CreatePlayer` -1))

(fn `SpawnDefaultPawnFor`
  (params (NewPlayer :type "Controller Object Reference") (StartSpot :type "Actor Object Reference"))
  (returns (ReturnValue :type "Pawn Object Reference"))
  (if (== (`GameplayStatics.GetPlayerControllerID` (`PlayerState.GetPlayerController` (`Controller.PlayerState` NewPlayer))) 0)
    (bind _returnvalue (`|SpawnActorFromClass` "/Game/GameBlueprints/Characters/PlayerCharacters/BP_MeleePlayerCharacter_RH.BP_MeleePlayerCharacter_RH_C" (`self.GetTransform` StartSpot) "Undefined" "MultiplyWithRoot" null null))
    (`Controller.Possess` NewPlayer _returnvalue)
    (else
      (bind _returnvalue_2 (`|SpawnActorFromClass` "/Game/GameBlueprints/Characters/PlayerCharacters/BP_RangePlayerCharacter_RH.BP_RangePlayerCharacter_RH_C" (`self.GetTransform` StartSpot) "Undefined" "MultiplyWithRoot" null null))
      (`Controller.Possess` NewPlayer _returnvalue_2)))
  (return _returnvalue_2))

(fn `UserConstructionScript`)